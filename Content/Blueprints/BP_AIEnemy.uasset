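; Zombie enemy for a VR game that wanders, chases seen pawns, attacks and dies with a random fall animation.
; Roaming loops AIMoveTo to random nearby points; PawnSensing switches to chase and attack montage, with a retriggerable delay resuming roaming.
; An attack collider, toggled by CollisionOn/CollisionOff events, deals random damage to VRPawn.
; Incoming damage is debounced before reducing HP and playing blood and hit reactions.
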(event `self.ReceiveBeginPlay`
  (`self.Move`)
  (`PrimitiveComponent.SetCollisionEnabled` (`self.AttackCollision`) "NoCollision"))

(event `Move`
  (if (not (or (`self.isdead`) (`self.Seeplayer?`))) :!label _label
    (`|AIMoveTo` self (`NavigationSystemV1.K2_GetRandomReachablePointInRadius` (`self.K2_GetActorLocation`) 500.0 null null) null
      (:`OnSuccess`
        (`KismetSystemLibrary.Delay` 2.0)
        (goto _label)))))

(event `self.PawnSensing.OnSeePawn`
  (params (Pawn :type "Pawn Object Reference"))
  (if (not (`self.isdead`))
    (set `self.Seeplayer?` true)
    (`|ExecutionSequence`
      (:`then_0`
        (`|AIMoveTo` self (0.0 0.0 0.0) Pawn
          (:`OnSuccess`
            (`/Engine/EditorBlueprintResources/StandardMacros.DoOnce` false :!label _label_2
              (:`Completed`
                (bind _returnvalue (`self.PlayAnimMontage` "/Game/Assets/Zonbi/Zombie_Z_Attack_Montage.Zombie_Z_Attack_Montage"))
                (`KismetSystemLibrary.Delay` _returnvalue)
                (goto _label_2 :!via `Reset`))))))
      (:`then_1`
        (`KismetSystemLibrary.RetriggerableDelay` 3.0)
        (set `self.Seeplayer?` false)
        (`self.Move`)))))

(event `self.ReceiveAnyDamage`
  (params (Damage :type "Float (single-precision)") (DamageType :type "DamageType Object Reference") (InstigatedBy :type "Controller Object Reference") (DamageCauser :type "Actor Object Reference"))
  (if (not (`self.isdead`))
    (`|ExecutionSequence`
      (:`then_0`
        (`/Engine/EditorBlueprintResources/StandardMacros.DoOnce` false :!label _label_3
          (:`Completed`
            (`ActorComponent.Activate` (`self.NS_Blood`) false)
            (set `self.HP` (- (`self.HP`) Damage))
            (`self.PlayAnimMontage` "/Game/Assets/Zonbi/Zombie_hitreaction_Montage.Zombie_hitreaction_Montage")
            (`KismetSystemLibrary.PrintString` (`KismetStringLibrary.Concat_StrStr` "残りHPは"))
            (if (< (`self.HP`) 0.0)
              (`/Engine/EditorBlueprintResources/StandardMacros.DoOnce` false
                (:`Completed`
                  (set `self.isdead` true)
                  (`MovementComponent.StopMovementImmediately` (`self.CharacterMovement`))
                  (`PrimitiveComponent.SetCollisionEnabled` (`self.CapsuleComponent`) "NoCollision")
                  (switch `int` (`KismetMathLibrary.RandomIntegerInRange` 0 1)
                    (:`0`
                      (`self.PlayAnimMontage` "/Game/Assets/Zonbi/Zombie_Z_FallingBack_Montage.Zombie_Z_FallingBack_Montage"))
                    (:`1`
                      (`self.PlayAnimMontage` "/Game/Assets/Zonbi/Zombie_Z_FallingForward_Montage.Zombie_Z_FallingForward_Montage")))))))))
      (:`then_1`
        (`KismetSystemLibrary.RetriggerableDelay` 0.07)
        (goto _label_3 :!via `Reset`)))))

(event `self.AttackCollision.OnComponentBeginOverlap`
  (params (OverlappedComponent :type "PrimitiveComponent Object Reference") (OtherActor :type "Actor Object Reference") (OtherComp :type "PrimitiveComponent Object Reference") (OtherBodyIndex :type Integer) (bFromSweep :type Boolean) (SweepResult :type "HitResult Structure (by ref)"))
  (bind _asvrpawn (cast `/Game/VRTemplate/Blueprints/VRPawn` OtherActor))
  (`GameplayStatics.ApplyDamage` _asvrpawn (`KismetMathLibrary.RandomFloatInRange` 0.1 0.2)))

(event `Collision On`
  (`PrimitiveComponent.SetCollisionEnabled` (`self.AttackCollision`) "QueryAndPhysics"))

(event `Collision Off`
  (`PrimitiveComponent.SetCollisionEnabled` (`self.AttackCollision`) "NoCollision"))

(fn `UserConstructionScript`)