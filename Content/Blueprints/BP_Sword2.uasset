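; Sword Blueprint that damages actors tagged "Zombi" through sphere traces along its blade.
; BeginPlay caches the blade's TraceStart and TraceEnd socket locations and sets the trace radius from their distance.
; Each Tick loops over interpolation steps between the sockets, tracing toward the cached locations to cover movement between frames.
; The cache refreshes inside the loop after every trace, and each valid tagged hit applies damage without duplicate filtering.
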(event `self.ReceiveBeginPlay`
  (`self.CacheTraceLocation`)
  (set `self.TraceStep` (/ (`KismetMathLibrary.Vector_Distance` (`self.LastTraceStartLocation`) (`self.LastTraceEndLocation`)) 20.0)))

(event `self.ReceiveTick`
  (params (DeltaSeconds :type "Float (single-precision)"))
  (bind _staticmesh (`self.StaticMesh`))
  (for _index (range 11)
    (bind _returnvalue (`KismetMathLibrary.Conv_IntToDouble` (/ _index 10)))
    (bind _outhit (`KismetSystemLibrary.SphereTraceSingle` (`KismetMathLibrary.VLerp` (`SceneComponent.GetSocketLocation` _staticmesh "TraceStart") (`SceneComponent.GetSocketLocation` _staticmesh "TraceEnd") _returnvalue) (`KismetMathLibrary.VLerp` (`self.LastTraceStartLocation`) (`self.LastTraceEndLocation`) _returnvalue) (`self.TraceStep`) "TraceTypeQuery1"))
    (`self.CacheTraceLocation`)
    (bind (_bblockinghit _binitialoverlap _time _distance _location _impactpoint _normal _impactnormal _physmat _hitactor) (`GameplayStatics.BreakHitResult` _outhit))
    (`/Engine/EditorBlueprintResources/StandardMacros.IsValid` _hitactor
      (:`Is Valid`
        (if (`self.ActorHasTag` _hitactor "Zombi")
          (`GameplayStatics.ApplyDamage` _hitactor 1.0 null null "/Script/Engine.DamageType"))))))

(event `CacheTraceLocation`
  (bind _staticmesh (`self.StaticMesh`))
  (set `self.LastTraceStartLocation` (`SceneComponent.GetSocketLocation` _staticmesh "TraceStart"))
  (set `self.LastTraceEndLocation` (`SceneComponent.GetSocketLocation` _staticmesh "TraceEnd")))

(fn `UserConstructionScript`)