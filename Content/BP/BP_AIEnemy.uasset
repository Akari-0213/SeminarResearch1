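; BP_AIEnemy is an enemy AI that wanders, chases pawns it sees and can be killed by damage.
; Move loops AI moves to random nearby reachable points, pausing after each success, while Seeplayer is false.
; PawnSensing sets Seeplayer and starts a chase, and a retriggerable delay resumes wandering after sightings stop.
; AnyDamage lowers HP, prints a label without the value, and destroys the actor below zero.
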(event `self.ReceiveBeginPlay`
  (`self.Move`))

(event `Move`
  (if (not (`self.Seeplayer?`)) :!label _label
    (`|AIMoveTo` self (`NavigationSystemV1.K2_GetRandomReachablePointInRadius` (`self.K2_GetActorLocation`) 500.0 null null) null
      (:`OnSuccess`
        (`KismetSystemLibrary.Delay` 2.0)
        (goto _label)))))

(event `self.PawnSensing.OnSeePawn`
  (params (Pawn :type "Pawn Object Reference"))
  (set `self.Seeplayer?` true)
  (`|ExecutionSequence`
    (:`then_0`
      (`|AIMoveTo` self (0.0 0.0 0.0) Pawn))
    (:`then_1`
      (`KismetSystemLibrary.RetriggerableDelay` 3.0)
      (set `self.Seeplayer?` false)
      (`self.Move`))))

(event `self.ReceiveAnyDamage`
  (params (Damage :type "Float (single-precision)") (DamageType :type "DamageType Object Reference") (InstigatedBy :type "Controller Object Reference") (DamageCauser :type "Actor Object Reference"))
  (set `self.HP` (- (`self.HP`) Damage))
  (`KismetSystemLibrary.PrintString` (`KismetStringLibrary.Concat_StrStr` "残りHPは"))
  (if (< (`self.HP`) 0.0)
    (`self.K2_DestroyActor`)))

(fn `UserConstructionScript`)